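; Spider character Blueprint from the full sample, relying on its parent class, with all event graph nodes left disabled.
; SetupHPBar casts the ACF health widget to CharacterInfo_WBP and initializes it with the spider itself.
; ShouldBeIgnored always returns false, and the construction script only calls the parent.
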(event EventBeginPlay
  (|CallParentFunction) ; This node is disabled and will not be called.\nDrag off pins to build functionality.
)

(event Collision|EventActorBeginOverlap
  (params (OtherActor :type Actor%20Object%20Reference))
  (|CallParentFunction OtherActor) ; This node is disabled and will not be called.\nDrag off pins to build functionality.
)

(event EventTick
  (params (DeltaSeconds :type Float%20%28single-precision%29))
  (|CallParentFunction DeltaSeconds) ; This node is disabled and will not be called.\nDrag off pins to build functionality.
)

(fn ConstructionScript
  (|CallParentFunction))

(fn SetupHPBar
  (bind _ascharacter_info_wbp (Utilities|Casting|CastToCharacterInfo_WBP (UserInterface|GetWidget (Variables|Default|GetACF%20HealthWidget))))
  (Default|InitCharacterInfo _ascharacter_info_wbp self))

(fn ShouldbeIgnored
  (return false))