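; ACFFullEnemyBP is an enemy character Blueprint in the Ascent Combat Framework full sample, with nearly all behavior inherited from its parent class.
; SetupHPBar casts the health widget component's widget to CharacterInfo_WBP and initializes it with this character.
; ShouldBeIgnored always returns false, and BeginPlay and the construction script only call their parent versions.
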(event EventBeginPlay
  (|CallParentFunction))

(event Collision|EventActorBeginOverlap
  (params (OtherActor :type Actor%20Object%20Reference))
  (|CallParentFunction OtherActor) ; This node is disabled and will not be called.\nDrag off pins to build functionality.
)

(fn ConstructionScript
  (|CallParentFunction))

(fn SetupHPBar
  (bind _ascharacter_info_wbp (Utilities|Casting|CastToCharacterInfo_WBP (UserInterface|GetWidget (Variables|Default|GetACF%20HealthWidget))))
  (Default|InitCharacterInfo _ascharacter_info_wbp self))

(fn ShouldbeIgnored
  (return false))