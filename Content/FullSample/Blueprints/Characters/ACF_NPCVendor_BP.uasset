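; ACF_NPCVendor_BP is an NPC vendor that opens a crafting UI when a pawn interacts with it.
; OnInteractedbyPawn casts the pawn's controller to PlayerController, creates the CraftingWidget for that player and adds it to the viewport.
; Input mode switch to UI-only and mouse cursor display are applied to player index 0, rather than to the interacting controller.
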(event EventBeginPlay
  (|CallParentFunction) ; This node is disabled and will not be called.\nDrag off pins to build functionality.
)

(event Collision|EventActorBeginOverlap
  (params (OtherActor :type Actor%20Object%20Reference))
  (|CallParentFunction OtherActor) ; This node is disabled and will not be called.\nDrag off pins to build functionality.
)

(event EventTick
  (params (DeltaSeconds :type Float%20%28single-precision%29))
  (|CallParentFunction DeltaSeconds) ; This node is disabled and will not be called.\nDrag off pins to build functionality.
)

(event EventOnInteractedbyPawn
  (params (Pawn :type Pawn%20Object%20Reference) (interactionType :type String))
  (bind _returnvalue (Game|GetPlayerController 0))
  (bind _asplayer_controller (Utilities|Casting|CastToPlayerController (Pawn|GetController Pawn)))
  (bind _returnvalue_2 (UserInterface|CreateWidget (Variables|Default|GetCraftingWidget) _asplayer_controller))
  (UserInterface|Viewport|AddtoViewport _returnvalue_2 0)
  (Input|SetInputModeUIOnly _returnvalue _returnvalue_2 "DoNotLock" false)
  (Variables|/Script/Engine.PlayerController|SetbShowMouseCursor _returnvalue true))

(fn ConstructionScript
  (|CallParentFunction))