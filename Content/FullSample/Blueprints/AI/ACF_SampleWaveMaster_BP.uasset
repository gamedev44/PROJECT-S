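; Sample wave master actor that runs an AI enemy wave through its WavesComp and announces progress on screen.
; On BeginPlay, the authority adds a spider agent to the first wave and starts it.
; The component's wave-started and all-waves-ended events feed a shared SpawnWidget event, which shows a timed message widget to the first player controller.
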(event OnWaveStarted(wavesComp)
  (params (waveIndex :type Integer))
  (bind _result (Math|Integer|IncrementInt waveIndex)
    (:%20%20
      (CallFunction|SpawnWidget (Utilities|Text|ToText(String) (Utilities|String|Append "WAVE STARTED:  " (Utilities|String|ToString(Integer) _result))) 5.0))))

(event OnAllWavesEnded(wavesComp)
  (CallFunction|SpawnWidget "ALL WAVES COMPLETED!!" 5.0))

(event Custom|SpawnWidget
  (params (InMessage :type Text) (Duration :type Float%20%28single-precision%29))
  (bind _returnvalue (UserInterface|CreateWidget "/Game/FullSample/UI/ACF_OnScreenMessage_WBP.ACF_OnScreenMessage_WBP_C" (Game|GetPlayerController 0) InMessage Duration))
  (UserInterface|Viewport|AddtoPlayerScreen _returnvalue))

(event EventBeginPlay
  (|CallParentFunction)
  (if (Ability|HasAuthority)
    (Class|ACFAIWavesMasterComponent|AddAgenttoWave (Variables|Default|GetwavesComp) 0 "/Game/FullSample/Blueprints/Characters/Spider/ACFFullSpiderBP.ACFFullSpiderBP_C" 1)
    (Class|ACFAIWavesMasterComponent|StartWave (Variables|Default|GetwavesComp))))

(event Collision|EventActorBeginOverlap
  (params (OtherActor :type Actor%20Object%20Reference)))

(event EventTick
  (params (DeltaSeconds :type Float%20%28single-precision%29)))

(fn ConstructionScript)