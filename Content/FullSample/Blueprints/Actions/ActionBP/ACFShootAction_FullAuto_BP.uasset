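; Full-auto shoot action for the Ascent Combat Framework that fires the character's equipped ranged weapon continuously.
; It caches the current main weapon from the equipment component and can only execute while that weapon can shoot.
; Each time the looping action hits its notable point, it fires a projectile or swipe trace per the weapon's shooting type, releasing the action once shooting is no longer possible.
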(event EventOnActionStarted
  (params (contextString :type String))
  (|CallParentFunction contextString)
  (CallFunction|SetWeaponVars (Variables|Default|GetCharacterOwner)))

(event EventOnNotablePointReached
  (bind _as_acfranged_weapon (Variables|Default|GetAs%20ACFRanged%20Weapon))
  ;[1 1 1] This will trigger repeatedly when we're looping.
  (|CallParentFunction)
  (if (Class|ACFRangedWeapon|CanShoot (Variables|Default|GetAs%20ACFRanged%20Weapon))
    (switch Utilities|FlowControl|Switch|SwitchonEShootingType (Variables|/Script/InventorySystem.ACFRangedWeapon|GetShootingType _as_acfranged_weapon)
      (:EProjectile
        (Class|ACFRangedWeapon|ShootProjectile _as_acfranged_weapon (Variables|Default|GetTarget%20Type) 1.0 (Variables|Default|GetProjectile%20Override)))
      (:ESwipeTrace
        (Class|ACFRangedWeapon|SwipeTraceShoot _as_acfranged_weapon (Variables|Default|GetTarget%20Type))))
    (else
      (Class|ACFSustainedAction|ReleaseAction))))

(fn SetWeaponVars
  (params (Target :type Actor%20Object%20Reference))
  (bind _returnvalue (Actor|GetComponentbyClass Target "/Script/InventorySystem.ACFEquipmentComponent"))
  (bind _returnvalue_2 (Class|ACFEquipmentComponent|GetCurrentMainWeapon _returnvalue))
  (Utilities|IsValid _returnvalue
    (:Is%20Valid
      (Utilities|IsValid _returnvalue_2
        (:Is%20Valid
          (bind _asacfranged_weapon (Utilities|Casting|CastToACFRangedWeapon _returnvalue_2))
          (bind _output_get (Variables|Default|SetAs%20ACFRanged%20Weapon _asacfranged_weapon)))))))

(fn CanExecuteAction
  (params (owner :type Character%20Object%20Reference))
  (bind _as_acfranged_weapon (Variables|Default|GetAs%20ACFRanged%20Weapon))
  (CallFunction|SetWeaponVars owner)
  (Utilities|IsValid _as_acfranged_weapon
    (:Is%20Valid
      (return (Class|ACFRangedWeapon|CanShoot _as_acfranged_weapon)))
    (:Is%20Not%20Valid
      (return false))))