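; Interactable save-point actor that saves the game world when a pawn interacts with it.
; Interaction calls the ALS load-and-save subsystem's SaveGameWorld with a slot name, then prints the success result from the callback.
; CanBeInteracted blocks saving while the ACF game state is in battle, printing a warning, and the interactable name is "SaveGame".
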(event Custom|OnWorldSaved
  (params (Success :type Boolean))
  ;[1 1 1] On Load, Make sure to load the slot name selected here. Left it hard coded as example, implementation will depend on design choice of each game
  (Development|PrintString (Utilities|String|ToString(Boolean) Success) true true "(R=0.000000,G=0.660000,B=1.000000,A=1.000000)" 2e+01))

(event EventBeginPlay)

(event Collision|EventActorBeginOverlap
  (params (OtherActor :type Actor%20Object%20Reference)))

(event EventTick
  (params (DeltaSeconds :type Float%20%28single-precision%29)))

(event EventOnInteractedbyPawn
  (params (Pawn :type Pawn%20Object%20Reference) (interactionType :type String))
  ;[1 1 1] On Load, Make sure to load the slot name selected here. Left it hard coded as example, implementation will depend on design choice of each game
  (Class|ALSLoadandSaveSubsystem|SaveGameWorld (Subsystems|GetALSLoadandSaveSubsystem) (Variables|Default|GetSlot%20Name) (delegate Custom|OnWorldSaved) true true))

(fn ConstructionScript)

(fn CanbeInteracted
  (params (Pawn :type Pawn%20Object%20Reference))
  (bind _returnvalue (Class|ACFFunctionLibrary|GetACFGameState))
  (bind _returnvalue_2 (Class|ACFGameState|GetBattleState _returnvalue))
  (bind _returnvalue_3 (Utilities|Enum|NotEqual(Enum) _returnvalue_2 "EBattle"))
  (if _returnvalue_3
    (return _returnvalue_3)
    (else
      (Development|PrintString "CAN'T SAVE WHILE IN BATTLE!")
      (return false))))

(fn GetInteractableName
  (return "SaveGame"))