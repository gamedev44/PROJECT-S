(event EventBeginPlay
  (|CallParentFunction))

(event EventTick
  (params (DeltaSeconds :type Float%20%28single-precision%29))
  (|CallParentFunction DeltaSeconds) ; This node is disabled and will not be called.\nDrag off pins to build functionality.
)

(event Input|KeyboardEvents|DebugKeyI
  (params (Key :type Key%20Structure) (ActionValue :type Input%20Action%20Value%20Structure))
  (:Pressed
    (CallFunction|HandleInventory)))

(event Input|KeyboardEvents|DebugKeyJ
  (params (Key :type Key%20Structure) (ActionValue :type Input%20Action%20Value%20Structure))
  (:Pressed
    (CallFunction|HandleStat)))

(fn ConstructionScript
  (|CallParentFunction))

(fn HandleStat
  (Utilities|FlowControl|FlipFlop
    (:A
      (bind _returnvalue (UserInterface|CreateWidget "/AscentCombatFramework/ARSStatistics/UI/ARSStatisticInfo.ARSStatisticInfo_C" self (Class|ACFCharacter|GetStatisticsComponent (Class|ACFPlayerController|GetPossessedACFCharacter))))
      (bind _output_get (Variables|Default|SetStatInfo _returnvalue))
      (UserInterface|Viewport|AddtoViewport _output_get 0))
    (:B
      (Widget|RemovefromParent (Variables|Default|GetStatInfo)))))

(fn HandleInventory
  (Utilities|IsValid (Variables|Default|GetWBP_Inventory)
    (:Is%20Valid
      (if (UserInterface|Viewport|IsinViewport (Variables|Default|GetWBP_Inventory))
        (Utilities|IsValid (Variables|Default|GetWBP_Inventory)
          (:Is%20Valid
            (Widget|RemovefromParent (Variables|Default|GetWBP_Inventory))
            (Variables|Default|SetbShowMouseCursor false)
            (Input|SetInputModeGameOnly self false)))
        (else
          (Utilities|IsValid (Variables|Default|GetWBP_Inventory) :!label _label
            (:Is%20Valid
              _)
            (:Is%20Not%20Valid
              (bind _returnvalue (UserInterface|CreateWidget "/Game/FullSample/UI/Inventory/WBP_Inventory.WBP_Inventory_C" self))
              (Variables|Default|SetWBP_Inventory _returnvalue)))
          (UserInterface|Viewport|AddtoViewport (Variables|Default|GetWBP_Inventory) 0)
          (Variables|Default|SetbShowMouseCursor true)
          (Input|SetInputModeGameandUI self (Variables|Default|GetWBP_Inventory) "DoNotLock" true false))))
    (:Is%20Not%20Valid
      (goto _label))))